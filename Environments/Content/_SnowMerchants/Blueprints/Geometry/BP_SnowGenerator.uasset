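; BP_SnowGenerator is a Geometry Script generated-mesh actor that builds a procedural snow layer on listed static mesh actors.
; On rebuild it copies each mesh into a world-space compute mesh, then raycasts down from random seeded points using a BVH.
; Each hit appends a sphere box, and the result moves to actor space.
; Optional SDF morphology and smoothing blend it into snow; the UV and normals pass is disconnected.
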(event `self.OnRebuildGeneratedMesh`
  (params (TargetMesh :type "DynamicMesh Object Reference"))
  (bind _sphereraycaststream (`self.SphereRaycastStream`))
  (set `self.TargetMesh` TargetMesh)
  ;[1 1 1] Reset Raycast Mesh Actors
  (`KismetArrayLibrary.Array_Clear` (`self.RaycastMeshActors`))
  (`|ExecutionSequence`
    (:`then_0`
      ;[1 1 1] Create Temp Compute Meshes for All Meshes to Add Snow To
      ;;[1 1 1] Iterate through every mesh
      (for _array_element (`self.MeshesToAddSnowTo`)
        ;;[1 1 1] Allocate Compute Mesh
        (bind _returnvalue (`self.AllocateComputeMesh`))
        (`KismetArrayLibrary.Array_Add` (`self.RaycastMeshActors`) _returnvalue)
        ;;[1 1 1] Copy mesh to the new compute mesh
        (`GeometryScriptLibrary_SceneUtilityFunctions.CopyMeshFromComponent` (`Actor.RootComponent` (break `/Game/_SnowMerchants/Blueprints/Geometry/BPS_MeshesToAddSnowTo` _array_element)) _returnvalue (struct) true null)))
    (:`then_1`
      ;[1 1 1] Create snow spheres for each compute mesh
      (for (_array_element_2 _array_index) (`self.RaycastMeshActors`)
        (bind _output_get (set `self.CurrentRaycastMeshActor` _array_element_2))
        (bind (_outputbvh _returnvalue_2) (`GeometryScriptLibrary_MeshSpatial.BuildBVHForMesh` _output_get null))
        (set `self.OutputBVH` _outputbvh)
        (bind (_output_staticmeshactor _output_numsnowspheres) (break `/Game/_SnowMerchants/Blueprints/Geometry/BPS_MeshesToAddSnowTo` (`|GetArrayItem` (`self.MeshesToAddSnowTo`) _array_index)))
        (for _ (range 1 (+ _output_numsnowspheres 1))
          (bind (_min _max) (break `Box` (`GeometryScriptLibrary_MeshQueryFunctions.GetMeshBoundingBox` _returnvalue_2)))
          ;;[1 1 1] Create Snow Spheres
          ;;;[1 1 1] Calculate raycast intersection with mesh
          (bind _hitresult (`GeometryScriptLibrary_MeshSpatial.FindNearestRayIntersectionWithMesh` (`self.CurrentRaycastMeshActor`) (`self.OutputBVH`) (`KismetMathLibrary.MakeVector` (`KismetMathLibrary.RandomFloatInRangeFromStream` _sphereraycaststream (.x _min) (.x _max)) (`KismetMathLibrary.RandomFloatInRangeFromStream` _sphereraycaststream (.y _min) (.y _max)) (+ (.z _max) 50.0)) (0.0 0.0 -1.0) (struct) null)
            (:`Found`
              ;;;[1 1 1] Create snow sphere at intersection point
              (`GeometryScriptLibrary_MeshPrimitiveFunctions.AppendSphereBox` (`self.TargetMesh`) (struct) (`KismetMathLibrary.MakeTransform` (`.HitPosition` (break `GeometryScriptRayHitResult` _hitresult))) 10.0 6 6 6 "Center" null))))
        ;;[1 1 1] Release the current ComputeMesh after generating snow
        (`self.ReleaseComputeMesh` (`self.CurrentRaycastMeshActor`))))
    (:`then_2`
      ;[1 1 1] Transform the mesh to position the snow correctly
      (`GeometryScriptLibrary_MeshTransformFunctions.TransformMesh` (`self.TargetMesh`) (`KismetMathLibrary.InvertTransform` (`self.GetTransform`)) true null)
      ;[1 1 1] Apply extra to make the snow look more like snow!
      ;;[1 1 1] Remesh the snow
      (if (`self.Remesh`)
        (bind _returnvalue_3 (`GeometryScriptLibrary_MeshVoxelFunctions.ApplyMeshMorphology` (`self.TargetMesh`) (make `GeometryScriptMorphologyOptions` (make `GeometryScript3DGridParameters` "GridResolution" 0.5 32) false (make `GeometryScript3DGridParameters` "GridResolution") "Dilate" (`self.SnowThickness`)) null))
        ;;[1 1 1] Smooth the snow mesh
        (bind _returnvalue_4 (`GeometryScriptLibrary_MeshDeformFunctions.ApplyIterativeSmoothingToMesh` _returnvalue_3 (struct) (make `GeometryScriptIterativeMeshSmoothingOptions` (`self.SnowSmoothnessStrength`)) null))))
    (:`then_3`
      ;[1 1 1] Reset the procedural snow system
      ;;[1 1 1] Reset Raycast Mesh Actors
      (`KismetArrayLibrary.Array_Clear` (`self.RaycastMeshActors`))
      (set `self.OutputBVH` (struct))
      (set `self.CurrentRaycastMeshActor` null))))

(fn `UserConstructionScript`)